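; Environment Blueprint that runs a looping chase effect along wall lights, showing one pair at a time.
; At BeginPlay it hides every Wall_Light overlapping it, pairs those with world X within PairTolerance into an array sorted by ascending X, then disables the Trigger's collision.
; An endless delay loop hides the current pair and shows the next, wrapping around, by toggling actor visibility at BlinkDelay intervals.
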(event Custom|BlinkLights
  (CallFunction|ShowCurrentLightPair false :!label _label)
  (Variables|State|SetLitIndex (Math|Integer|%(Integer) (+ (Variables|State|GetLitIndex) 1) (Utilities|Array|Length (Variables|State|GetLightData))))
  (CallFunction|ShowCurrentLightPair true)
  (Utilities|FlowControl|Delay (Variables|Config|GetBlinkDelay))
  (goto _label))

(event EventBeginPlay
  (CallFunction|GatherLights)
  (Collision|SetCollisionEnabled (Variables|Default|GetTrigger) "NoCollision") ; Turn off collision after we have\ngathered all the lights
  (Variables|State|SetLitIndex (Utilities|Array|LastIndex (Variables|State|GetLightData)))
  (CallFunction|BlinkLights))

(fn ConstructionScript)

(fn GatherLights
  (bind _output_get (LocalVariables|SetLights (Collision|GetOverlappingActors "/Game/Modular_Sewer_Pack_Survival_Edition/Blueprints/Wall_Light.Wall_Light_C" :!class /Script/Engine.Actor)))
  (for _array_element _output_get
    (Rendering|SetActorHiddenInGame _array_element true) ; Hide the light
    (CallFunction|AddLight (Math|Float|Round (.X (Math|Vector|BreakVector (Transformation|GetActorLocation _array_element)))) (.AsWall%20Light (Utilities|Casting|CastToWall_Light _array_element)))))

(fn AddLight
  (params (CoordinateX :type Integer) (Light :type Wall%20Light%20Object%20Reference))
  (for (_array_element _array_index) (Variables|State|GetLightData)
    (if (<= (Math|Integer|Absolute(Integer) (- (Utilities|Struct|BreakSBlinkingLight _array_element) CoordinateX)) (Variables|Constant|GetPairTolerance)) ; We have already found\nthe pair or this light
      (Utilities|Struct|SetmembersinSBlinkingLight (Utilities|Array|Get(acopy) (Variables|State|GetLightData) _array_index) Light) ; Set the pair of the existing light
      (return)
      (elif (> (Utilities|Struct|BreakSBlinkingLight _array_element) CoordinateX) ; We have found the spot in\nthe middle of the array
        (Utilities|Array|Insert (Variables|State|GetLightData) (Utilities|Struct|MakeSBlinkingLight CoordinateX Light) _array_index) ; Insert it to its place
        (return))))
  (Utilities|Array|Add (Variables|State|GetLightData) (Utilities|Struct|MakeSBlinkingLight CoordinateX Light)) ; Didn't find its place, add it to the end
)

(fn ShowCurrentLightPair
  (params (bVisible :type Boolean))
  (LocalVariables|SetLightPair (Utilities|Array|Get(acopy) (Variables|State|GetLightData) (Variables|State|GetLitIndex)))
  (Rendering|SetActorHiddenInGame (Utilities|Struct|BreakSBlinkingLight (LocalVariables|GetLightPair)) (not bVisible))
  (Rendering|SetActorHiddenInGame (Utilities|Struct|BreakSBlinkingLight (LocalVariables|GetLightPair)) (not bVisible)))