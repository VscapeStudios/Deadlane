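; Action volume Blueprint that triggers a configured list of actors when it fires for a kart.
; Firing loops over ActionActors and sends OnActionFiredMessage, with the action tag and instigating kart, to each one implementing BI_ActionVolumeTriggerable.
; CanFire refuses when the actor list is empty and otherwise defers to the parent's check.
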(event EventBeginPlay
  (|CallParentFunction) ; This node is disabled and will not be called.\nDrag off pins to build functionality.
)

(event Collision|EventActorBeginOverlap
  (params (OtherActor :type Actor%20Object%20Reference))
  (|CallParentFunction OtherActor) ; This node is disabled and will not be called.\nDrag off pins to build functionality.
)

(event EventTick
  (params (DeltaSeconds :type Float%20%28single-precision%29))
  (|CallParentFunction DeltaSeconds) ; This node is disabled and will not be called.\nDrag off pins to build functionality.
)

(event EventFireAction
  (params (InstigatorKart :type DE%20Ghost%20Kart%20Object%20Reference))
  (for _array_element (Variables|Default|GetActionActors)
    (if (Utilities|DoesObjectImplementInterface _array_element "/Game/DeadEnd/Blueprints/ActionVolume/BI_ActionVolumeTriggerable.BI_ActionVolumeTriggerable_C")
      (Class|BIActionVolumeTriggerable|OnActionFired(Message) _array_element (Variables|Default|GetActionTag) InstigatorKart))))

(fn ConstructionScript
  (|CallParentFunction))

(fn CanFire
  (params (OverlappingKart :type DE%20Ghost%20Kart%20Object%20Reference))
  (if (> (Utilities|Array|Length (Variables|Default|GetActionActors)) 0)
    (return (|CallParentFunction OverlappingKart))
    (else
      (return false))))