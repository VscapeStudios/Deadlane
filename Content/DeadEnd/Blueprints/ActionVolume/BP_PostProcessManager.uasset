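; Post-process manager that plays "Telly" screen effects in response to kart action events, registering itself with DeadEnd_GameState on BeginPlay.
; OnActionFired routes action tags: Go Crazy and Go Sleep use timelines to animate blend weights on two post-process components.
; Glitch runs parallel timelines driving Cham's pixel dissolve and glitch parameters, switching each off shortly after finishing.
; The victim kart is passed through but does not target the effect.
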(event Custom|StartTellyGlitch
  (params (VictimKart :type DE%20Ghost%20Kart%20Object%20Reference))
  ;[1 1 1] Telly Glith
  (Utilities|IsValid (Variables|Default|GetCham)
    (:Is%20Valid
      (Utilities|FlowControl|Sequence
        (:then_0
          ;;[0 0 0] PixelDissolve
          (bind _newtrack_0 (Timeline|Timeline_2 PlayFromStart)
            (:Update
              (Variables|/Game/Chameleon/Chameleon.Chameleon_C|SetPixel%20Dissolve%20Intensity (Variables|Default|GetCham) _newtrack_0)
              (Default|PixelDissolveFunc (Variables|Default|GetCham) true))
            (:Finished
              (Utilities|FlowControl|Delay 0.2)
              (Default|PixelDissolveFunc (Variables|Default|GetCham) false))))
        (:then_1
          ;;[0 0 0] Glitch
          (bind (_direction _glitch_speed _glitch_lines _glitch_blocking _glitch_grid_distortion_power _glitch_grid_distortion_size _glitch_grid_distortion_speed) (Timeline|Timeline_3 PlayFromStart)
            (:Update
              (Utilities|FlowControl|Sequence
                (:then_0
                  (Variables|/Game/Chameleon/Chameleon.Chameleon_C|SetGlitch%20Speed (Variables|Default|GetCham) _glitch_speed)
                  (Variables|/Game/Chameleon/Chameleon.Chameleon_C|SetGlitch%20Lines (Variables|Default|GetCham) _glitch_lines)
                  (Variables|/Game/Chameleon/Chameleon.Chameleon_C|SetGlitch%20Blocking (Variables|Default|GetCham) _glitch_blocking))
                (:then_1
                  (Variables|/Game/Chameleon/Chameleon.Chameleon_C|SetGlitch%20Grid%20Distortion%20Power (Variables|Default|GetCham) _glitch_grid_distortion_power)
                  (Variables|/Game/Chameleon/Chameleon.Chameleon_C|SetGlitch%20Grid%20Distortion%20Size (Variables|Default|GetCham) _glitch_grid_distortion_size)
                  (Variables|/Game/Chameleon/Chameleon.Chameleon_C|SetGlitch%20Grid%20Distortion%20Speed (Variables|Default|GetCham) _glitch_grid_distortion_speed))
                (:then_2
                  (Default|GlitchFunc (Variables|Default|GetCham) true))))
            (:Finished
              (Utilities|FlowControl|Delay 0.2)
              (Default|GlitchFunc (Variables|Default|GetCham) false))))))))

(event EventBeginPlay
  (bind _asdead_end_game_state (Utilities|Casting|CastToDeadEnd_GameState (Game|GetGameState)))
  (Default|RegisterPPManager _asdead_end_game_state self))

(event EventOnActionFired
  (params (ActionTag :type Name :default "None") (InstigatorKart :type DE%20Ghost%20Kart%20Object%20Reference))
  (bind _output_get (Variables|Default|SetInstigatorKart InstigatorKart))
  (Utilities|IsValid _output_get
    (:Is%20Valid
      (Development|PrintString (Utilities|String|Append "New Action: " (Utilities|String|ToString(Name) ActionTag)) false)
      (switch name ActionTag
        (:TellyGoCrazy
          (bind _newtrack_0 (Timeline|Timeline_0 PlayFromStart)
            (:Update
              (Variables|/Script/Engine.PostProcessComponent|SetBlendWeight (Variables|Default|GetPostProcess1) _newtrack_0))))
        (:TellyGoSleep
          (bind (_direction _newtrack_0_2 _newtrack_1) (Timeline|Timeline_1 PlayFromStart)
            (:Update
              (Variables|/Script/Engine.PostProcessComponent|SetBlendWeight (Variables|Default|GetPostProcess2) _newtrack_0_2)
              (Variables|/Script/Engine.PostProcessComponent|SetBlendWeight (Variables|Default|GetPostProcess1) _newtrack_1))))
        (:TellyGlitch
          (CallFunction|StartTellyGlitch (Variables|Default|GetInstigatorKart)))))))

(fn ConstructionScript)