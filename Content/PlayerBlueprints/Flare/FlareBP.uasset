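; Flare projectile fired by a kart player, reporting hits on karts other than the shooter's to the DeadEnd game mode.
; Tick sweeps it forward until the game instance's max travel time, an overlap hit or HasCollided stops it.
; Stopping swaps the trail for a brief flare burst with explosion sound and disables collision.
; Afterwards, Tick grows the expansion sphere radius and destroys the actor if Lifetime is zero or less.
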(event Custom|onEndTravel
  ;[1 1 1] Begin/End Travelling
  (Audio|SpawnSoundAttached "/Game/Sounds/Kart_Sounds/GPExplosion_Cue.GPExplosion_Cue" (Variables|Default|GetFlare) "None" "0, 0, 0" "0, 0, 0" "KeepRelativeOffset" false 1.0 1.0 0.0 0 0)
  (Components|Activation|Deactivate (Variables|Default|GetTrail))
  (Components|Activation|Activate (Variables|Default|GetFlare) false)
  (Collision|SetCollisionEnabled (Variables|Default|GetExpansionCollider) "NoCollision")
  (Collision|SetActorEnableCollision false)
  (Utilities|FlowControl|Delay 0.2)
  (Components|Activation|Deactivate (Variables|Default|GetFlare)))

(event Custom|onBeginTravel
  ;[1 1 1] Begin/End Travelling
  (Components|Activation|Activate (Variables|Default|GetTrail) false))

(event EventBeginPlay
  (Components|Activation|Activate (Variables|Default|GetLaunchExplosion) false))

(event Collision|EventActorBeginOverlap
  (params (OtherActor :type Actor%20Object%20Reference))
  (bind _asdeghost_kart (Utilities|Casting|CastToDEGhostKart OtherActor))
  (bind _player (Default|GetPlayerbyPawn (.AsDead%20End%20Game%20Mode (Utilities|Casting|CastToDeadEnd_GameMode (Game|GetGameMode))) _asdeghost_kart))
  (if (not (== (.id _player) (Variables|Default|GetshooterID)))
    (Default|OnFlareHitPlayer (.AsDead%20End%20Game%20Mode (Utilities|Casting|CastToDeadEnd_GameMode (Game|GetGameMode))) (Variables|Default|GetshooterID) (.id _player))
    (CallFunction|StopTravelling)))

(event EventTick
  (params (DeltaSeconds :type Float%20%28single-precision%29))
  ;[0 0.1982 1] Update - Would be nicer to configure a state machine here
  (Variables|Default|SetlifetimeElapsed (+ DeltaSeconds (Variables|Default|GetlifetimeElapsed)))
  (if (Variables|Default|GetisTravelling)
    (CallFunction|MoveForward DeltaSeconds)
    (else
      (CallFunction|PostTravelUpdate DeltaSeconds))))

(fn ConstructionScript
  (CallFunction|StartTravelling))

(fn MoveForward
  (params (dt :type Float%20%28single-precision%29))
  (bind _returnvalue (Game|GetGameInstance))
  (bind _asdead_end_instance (Utilities|Casting|CastToDeadEnd_Instance _returnvalue))
  (LocalVariables|SetframeDistance (* dt (Variables|Default|GettravelSpeed)))
  (Utilities|IsValid _asdead_end_instance
    (:Is%20Valid
      (if (<= (Variables|Default|GetlifetimeElapsed) (Variables|/Game/PlayerBlueprints/DeadEnd_Instance.DeadEnd_Instance_C|GetmaxFlareTravelTime _asdead_end_instance))
        (Utilities|FlowControl|Sequence
          (:then_0
            (Transformation|AddLocalOffset (Variables|Default|Getroot) (Math|Vector|MakeVector (LocalVariables|GetframeDistance) 0.0 0.0) true false))
          (:then_1
            (Variables|Default|SetdistanceTravelled (+ (LocalVariables|GetframeDistance) (Variables|Default|GetdistanceTravelled)))))
        (else
          (CallFunction|StopTravelling))))))

(fn PostTravelUpdate
  (params (dt :type Float%20%28single-precision%29))
  (Components|Sphere|SetSphereRadius (Variables|Default|GetExpansionCollider) (+ (* dt (Variables|Default|GetexpansionRate)) (Variables|/Script/Engine.SphereComponent|GetSphereRadius (Variables|Default|GetExpansionCollider))) true)
  (if (>= 0.0 (Variables|Default|Getlifetime))
    (Actor|DestroyActor)))

(fn StopTravelling
  (Variables|Default|SetisTravelling false)
  (CallFunction|OnEndTravel))

(fn StartTravelling
  (CallFunction|OnBeginTravel)
  (Variables|Default|SetisTravelling true))

(fn HasCollided
  (params (hitActor :type Actor%20Object%20Reference))
  (Audio|SpawnSoundAttached "/Game/Sounds/Kart_Sounds/GPExplosion_Cue.GPExplosion_Cue" (Variables|Default|GetFlare) "None" "0, 0, 0" "0, 0, 0" "KeepRelativeOffset" false 1.0 1.0 0.0 0 0)
  (CallFunction|StopTravelling))

(fn GetShooter
  (return (Variables|Default|GetshooterID)))