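; BP_Telly is a racing hazard that chases and catches the first human-driven DEGhostKart to enter its trigger, ignoring karts with GrimPrix.
; After a delay, it homes on that kart via ProjectileMovement and activates player 0's mirror.
; Capsule overlap with the target applies the caught effect and hides Telly before removal; a chase timeout destroys it and switches the mirror off.
; SCTelly's State parameter tracks idle, triggered and caught.
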(event OnComponentBeginOverlap(Capsule)
  (params (OverlappedComponent :type Primitive%20Component%20Object%20Reference) (OtherActor :type Actor%20Object%20Reference) (OtherComp :type Primitive%20Component%20Object%20Reference) (OtherBodyIndex :type Integer) (bFromSweep :type Boolean) (SweepResult :type Hit%20Result%20Structure%20%28by%20ref%29))
  (bind _asdeghost_kart (Utilities|Casting|CastToDEGhostKart OtherActor))
  (if (Math|Boolean|ANDBoolean (Variables|Default|GetbChasing) (== _asdeghost_kart (Variables|Default|GetTarget)) (not (Default|GetGrimPrix _asdeghost_kart)))
    (Utilities|FlowControl|Sequence
      (:then_0
        (Effects|Components|ParticleSystem|SetIntParameter (Variables|Default|GetSC_Telly) "State" 2) ; 0 - idle, 1 - triggered, 2 - caught
        (Development|PrintString (Utilities|String|Append "" (Utilities|String|ToString(Float) (- (Utilities|Time|GetGameTimeinSeconds) (Variables|Default|GetTriggerTime)))) true true "(R=1.000000,G=0.000000,B=0.097826,A=1.000000)")
        (Game|Components|ProjectileMovement|StopSimulating (Variables|Default|GetProjectileMovement1) (Collision|MakeHitResult false false 0.0 0.0 "0, 0, 0" "0, 0, 0" "0,0,1" "0,0,1" 0 0))
        (Rendering|SetVisibility (Variables|Default|GetScene) false true)
        (Actor|SetLifeSpan 1.0))
      (:then_1
        (Default|OnTellyCaughtKart _asdeghost_kart (Variables|TellyConfig|GetTellyEffectTime))))))

(event OnComponentBeginOverlap(Trigger)
  (params (OverlappedComponent :type Primitive%20Component%20Object%20Reference) (OtherActor :type Actor%20Object%20Reference) (OtherComp :type Primitive%20Component%20Object%20Reference) (OtherBodyIndex :type Integer) (bFromSweep :type Boolean) (SweepResult :type Hit%20Result%20Structure%20%28by%20ref%29))
  (bind _asdeghost_kart (Utilities|Casting|CastToDEGhostKart OtherActor))
  (if (not (Default|GetGrimPrix _asdeghost_kart))
    (if (and (not (Pawn|IsBotControlled _asdeghost_kart)) (not (Variables|Default|GetbTriggered)))
      (Variables|Default|SetbTriggered true)
      (Variables|Default|SetTarget _asdeghost_kart)
      (Development|PrintString "")
      (Effects|Components|ParticleSystem|SetIntParameter (Variables|Default|GetSC_Telly) "State" 1) ; 0 - idle, 1 - triggered, 2 - caught
      (Utilities|FlowControl|Delay (Variables|TellyConfig|GetTriggerDelay))
      (Transformation|SetActorRelativeRotation "0,100.000000, 0")
      (CallFunction|StartChasing)
      (Components|Animation|PlayAnimation (Variables|Default|GetSkeletalMesh) "/Game/Travel_Idle_Start.Travel_Idle_Start" false)
      (Components|Animation|PlayAnimation (Variables|Default|GetSkeletalMesh) "/Game/LifeLock_Fire.LifeLock_Fire" false))))

(event EventBeginPlay
  (Utilities|FlowControl|Sequence
    (:then_0
      ;[1 1 1] Set Apperance
      (bind _entrance (Timeline|Timeline_1 Play)
        (:Update
          (Rendering|Material|SetScalarParameterValueonMaterials (Variables|Default|GetSkeletalMesh) "Apperance" _entrance))))
    (:then_1
      ;[1 1 1] ApplyConfigs
      (Variables|/Script/Engine.ProjectileMovementComponent|SetHomingAccelerationMagnitude (Variables|Default|GetProjectileMovement1) (Variables|TellyConfig|GetHomingMagnitude))
      (Variables|/Script/Engine.ProjectileMovementComponent|SetMaxSpeed (Variables|Default|GetProjectileMovement1) (Variables|TellyConfig|GetMaxSpeed))
      (Actor|SetLifeSpan 0.0)
      (Effects|Components|ParticleSystem|SetIntParameter (Variables|Default|GetSC_Telly) "State" 0) ; 0 - idle, 1 - triggered, 2 - caught
    )))

(event Collision|EventActorBeginOverlap
  (params (OtherActor :type Actor%20Object%20Reference)))

(fn ConstructionScript
  (bind _returnvalue (Rendering|Material|CreateDynamicMaterialInstance (Variables|Default|GetSkeletalMesh) 1 "/Game/Models/Telly/Materials/M_VHS_Ghost_Insttelly.M_VHS_Ghost_Insttelly" "None" :!class /Script/Engine.PrimitiveComponent))
  (Variables|Default|SetDynamic%20Material _returnvalue))

(fn StartChasing
  (Utilities|IsValid (Variables|Default|GetTarget)
    (:Is%20Valid
      (Variables|Default|SetbChasing true)
      (Variables|/Script/Engine.ProjectileMovementComponent|SetbIsHomingProjectile (Variables|Default|GetProjectileMovement1) true)
      (Variables|/Script/Engine.ProjectileMovementComponent|SetHomingTargetComponent (Variables|Default|GetProjectileMovement1) (Variables|/Script/Engine.Actor|GetRootComponent (Variables|Default|GetTarget)))
      (Variables|Default|SetTriggerTime (Utilities|Time|GetGameTimeinSeconds))
      (bind _returnvalue (Utilities|Time|SetTimerbyFunctionName 0 "OnChasingTimerExpired" (Variables|TellyConfig|GetMaxChasingTime)))
      (Variables|Default|SetChasingTimer _returnvalue)
      (bind _asdeghost_kart (Utilities|Casting|CastToDEGhostKart (Game|Player|GetPlayerPawn 0)))
      (Default|SetMirrorActive _asdeghost_kart true))))

(fn OnChasingTimerExpired
  (Development|PrintString "")
  (Actor|DestroyActor)
  (Default|CallOnTellyLoseTarget)
  (bind _asdeghost_kart (Utilities|Casting|CastToDEGhostKart (Game|Player|GetPlayerPawn 0)))
  (Default|SetMirrorActive _asdeghost_kart false))