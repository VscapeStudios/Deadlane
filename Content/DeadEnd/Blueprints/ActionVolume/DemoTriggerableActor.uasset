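; Demo actor for the Telly character that reacts to tagged actions fired with an instigating kart.
; Wake Up plays a look-up montage and blast during a camera cutaway, eased from the kart's camera by timeline and aimed on Tick, then restores the view.
; Go Crazy attaches Telly, lerps it toward the kart, then plays a sound and destroys it; Go Sleep restores its rest transform.
; Ghost-material fade logic is unwired.
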(event EventBeginPlay
  (Variables|Default|SetRestTransform (Transformation|GetActorTransform)))

(event EventOnActionFired
  (params (ActionTag :type Name :default "None") (InstigatorKart :type DE%20Ghost%20Kart%20Object%20Reference))
  (bind _output_get (Variables|Default|SetInstigatorKart InstigatorKart))
  (Utilities|IsValid _output_get
    (:Is%20Valid
      (Development|PrintString (Utilities|String|Append "New Action: " (Utilities|String|ToString(Name) ActionTag)) false)
      (switch name ActionTag
        (:TellyWakeUp
          (bind _asplayer_controller (Utilities|Casting|CastToPlayerController (Pawn|GetController (Variables|Default|GetInstigatorKart))))
          (Game|Player|SetViewTargetwithBlend _asplayer_controller self 0.0 "VTBlend_Linear" 0.0 false)
          (Utilities|FlowControl|Sequence
            (:then_0
              (bind _alpha (Timeline|CameraTimeline PlayFromStart)
                (:Update
                  (Variables|Default|SetInterpLocation (Math|Vector|Lerp(Vector) (Transformation|GetWorldLocation (Variables|/Game/PlayerBlueprints/GhostKart/DEGhostKart.DEGhostKart_C|GetMainCamera (Variables|Default|GetInstigatorKart))) (Transformation|GetWorldLocation (Variables|Default|GetCameraLocator)) _alpha)))
                (:Finished
                  (Utilities|FlowControl|Delay 2.0)
                  (bind _asplayer_controller_2 (Utilities|Casting|CastToPlayerController (Pawn|GetController (Variables|Default|GetInstigatorKart))))
                  (Game|Player|SetViewTargetwithBlend _asplayer_controller_2 (Variables|Default|GetInstigatorKart) 0.0 "VTBlend_Linear" 0.0 false))))
            (:then_1
              (Variables|Default|SetInterpCamera true))
            (:then_2
              (Animation|Montage|PlayMontage (Variables|Default|GetSkeletalMesh) "/Game/Characters/Telly/AM_LookUp.AM_LookUp"
                (:then
                  (Audio|PlaySound2D "/Game/Sounds/Kart_Sounds/GP_Blast.GP_Blast" 1.0 1.0 0.0 0 0))))))
        (:TellyGoCrazy
          (Transformation|AttachActorToActor (Variables|Default|GetInstigatorKart) "None" "KeepWorld" "KeepWorld" "KeepWorld" true)
          (bind _alpha_2 (Timeline|TellyCrazy Play)
            (:Update
              (Transformation|SetActorTransform (Math|Transform|Lerp(Transform) (Variables|Default|GetRestTransform) (Math|Transform|ComposeTransforms (Variables|Default|GetTellyCrazyRelativeTransform) (Transformation|GetActorTransform (Variables|Default|GetInstigatorKart))) _alpha_2))
              (Utilities|FlowControl|Delay 2.0)
              (Rendering|SetVisibility (Variables|Default|GetSkeletalMesh) true false)
              (Audio|SpawnSoundAttached "/Game/Sounds/Telly/Vocaroo_1nNYwUq9aLnW.Vocaroo_1nNYwUq9aLnW" 0 "None" "0, 0, 0" "0, 0, 0" "KeepRelativeOffset" false 1.5 1.0 0.0 0 0)
              (Utilities|FlowControl|Delay 0.05)
              (Actor|DestroyActor))))
        (:TellyGoSleep
          (Transformation|DetachFromActor "KeepWorld" "KeepWorld" "KeepWorld")
          (Transformation|SetActorTransform (Variables|Default|GetRestTransform))
          (Audio|PlaySound2D "/Game/Sounds/Telly/TellyAppears.TellyAppears" 1.0 1.0 0.0 0 0))))))

(event EventTick
  (params (DeltaSeconds :type Float%20%28single-precision%29))
  (if (Variables|Default|GetInterpCamera)
    (Transformation|SetWorldLocationAndRotation (Variables|Default|GetCamera) (Variables|Default|GetInterpLocation) (Math|Rotator|MakeRotfromX (- (Transformation|GetWorldLocation (Variables|Default|GetCameraTarget)) (Transformation|GetWorldLocation (Variables|Default|GetCamera)))) false false)))

(fn ConstructionScript)