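; BP_ActionVolume_SpawnParticles is an action volume whose action is spawning a particle effect.
; Its FireAction event spawns the ParticleTemplate emitter at ParticlesTransform composed with the actor's transform, so the offset is relative to the volume.
; Only location and rotation of the composed transform are applied; scale is not passed to the emitter.
; The graph contains no trigger logic of its own.
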(event EventBeginPlay
  (|CallParentFunction) ; This node is disabled and will not be called.\nDrag off pins to build functionality.
)

(event Collision|EventActorBeginOverlap
  (params (OtherActor :type Actor%20Object%20Reference))
  (|CallParentFunction OtherActor) ; This node is disabled and will not be called.\nDrag off pins to build functionality.
)

(event EventTick
  (params (DeltaSeconds :type Float%20%28single-precision%29))
  (|CallParentFunction DeltaSeconds) ; This node is disabled and will not be called.\nDrag off pins to build functionality.
)

(event EventFireAction
  (params (InstigatorKart :type DE%20Ghost%20Kart%20Object%20Reference))
  (bind _returnvalue (Transformation|GetActorTransform))
  (bind _particlestransform (Variables|Particles|GetParticlesTransform))
  (bind _returnvalue_2 (Math|Transform|ComposeTransforms _particlestransform _returnvalue))
  (bind (_location _rotation) (Math|Transform|BreakTransform _returnvalue_2))
  (Effects|SpawnEmitteratLocation (Variables|Particles|GetParticleTemplate) _location _rotation))

(fn ConstructionScript
  (|CallParentFunction))