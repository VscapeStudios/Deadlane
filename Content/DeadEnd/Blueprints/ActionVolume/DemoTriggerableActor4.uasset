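; Demo triggerable actor that brings a Telly character to life when an action volume fires a tagged action for an instigating kart.
; The Wake Up, Go Crazy and Go Sleep tags each unhide the actor, play an attached sound and a montage, then hide it on completion.
; A camera fly-to, kart attachment and transform blend remain as disconnected logic, so the Tick camera interpolation is never switched on here.
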(event EventBeginPlay
  (Variables|Default|SetRestTransform (Transformation|GetActorTransform)))

(event EventOnActionFired
  (params (ActionTag :type Name :default "None") (InstigatorKart :type DE%20Ghost%20Kart%20Object%20Reference))
  (bind _output_get (Variables|Default|SetInstigatorKart InstigatorKart))
  (Utilities|IsValid _output_get
    (:Is%20Valid
      (Development|PrintString (Utilities|String|Append "New Action: " (Utilities|String|ToString(Name) ActionTag)) false)
      (switch name ActionTag
        (:TellyWakeUp
          (Rendering|SetActorHiddenInGame false)
          (Audio|SpawnSoundAttached "/Game/Sounds/Telly/Telly_trigger.Telly_trigger" 0 "None" "0, 0, 0" "0, 0, 0" "KeepRelativeOffset" false 1.0 1.0 0.0 0 0)
          (Animation|Montage|PlayMontage 0 "/Game/Characters/Telly/AM_LookUp.AM_LookUp"
            (:OnCompleted
              (Rendering|SetActorHiddenInGame true))))
        (:TellyGoCrazy
          (Rendering|SetActorHiddenInGame false)
          (Audio|SpawnSoundAttached "/Game/Sounds/Telly/telly_yell2.telly_yell2" 0 "None" "0, 0, 0" "0, 0, 0" "KeepRelativeOffset" false 1.0 1.0 0.0 0 0)
          (Animation|Montage|PlayMontage 0 "/Game/Ultimate_Prepare_Montage.Ultimate_Prepare_Montage"
            (:OnCompleted
              (Rendering|SetActorHiddenInGame true))))
        (:TellyGoSleep
          (Rendering|SetActorHiddenInGame false)
          (Audio|SpawnSoundAttached "/Game/Sounds/Telly/Telly_trigger.Telly_trigger" 0 "None" "0, 0, 0" "0, 0, 0" "KeepRelativeOffset" false 1.0 1.0 0.0 0 0)
          (Animation|Montage|PlayMontage 0 "/Game/Recall_DarkAngelSkin_Montage.Recall_DarkAngelSkin_Montage"
            (:OnCompleted
              (Rendering|SetActorHiddenInGame true))))))))

(event EventTick
  (params (DeltaSeconds :type Float%20%28single-precision%29))
  (if (Variables|Default|GetInterpCamera)
    (Transformation|SetWorldLocationAndRotation (Variables|Default|GetCamera) (Variables|Default|GetInterpLocation) (Math|Rotator|MakeRotfromX (- (Transformation|GetWorldLocation (Variables|Default|GetCameraTarget)) (Transformation|GetWorldLocation (Variables|Default|GetCamera)))) false false)))

(fn ConstructionScript)