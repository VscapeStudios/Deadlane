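; Tree trap that falls when interaction is requested and, while activated, applies timed trap damage to ghost karts.
; A flag set at BeginPlay chooses whether tree hits or box overlaps trigger the damage.
; A timeline pitches the tree down from its original rotation, then starts a respawn timer.
; Respawn drives a dynamic material's visibility parameter, resets rotation while hidden, reverses the fade and deactivates the trap.
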(event OnComponentHit(Tree)
  (params (HitComponent :type Primitive%20Component%20Object%20Reference) (OtherActor :type Actor%20Object%20Reference) (OtherComp :type Primitive%20Component%20Object%20Reference) (NormalImpulse :type Vector :default "0, 0, 0") (Hit :type Hit%20Result%20Structure%20%28by%20ref%29))
  (if (and (Variables|Constant|GetApplyEffectByHit) (Variables|Default|GetbActivated))
    (bind _asdeghost_kart (Utilities|Casting|CastToDEGhostKart OtherActor))
    (Default|OnTakeTrapDamage _asdeghost_kart (Variables|Constant|GetTrapEffectTime))))

(event OnComponentBeginOverlap(Box)
  (params (OverlappedComponent :type Primitive%20Component%20Object%20Reference) (OtherActor :type Actor%20Object%20Reference) (OtherComp :type Primitive%20Component%20Object%20Reference) (OtherBodyIndex :type Integer) (bFromSweep :type Boolean) (SweepResult :type Hit%20Result%20Structure%20%28by%20ref%29))
  (if (and (not (Variables|Constant|GetApplyEffectByHit)) (Variables|Default|GetbActivated))
    (bind _asdeghost_kart (Utilities|Casting|CastToDEGhostKart OtherActor))
    (Default|OnTakeTrapDamage _asdeghost_kart (Variables|Constant|GetTrapEffectTime))))

(event Custom|RespawnTrap
  (bind (_direction _visibilityratio) (Timeline|VisibilityAnimation PlayFromStart)
    (:Update
      (Rendering|Material|SetScalarParameterValue (Variables|State|GetMaterial) "VisibilityRatio" _visibilityratio :!class /Script/Engine.MaterialInstanceDynamic))
    (:Finished
      (if (Utilities|Enum|Equal(Enum) _direction "Forward") ; Did it just disappear?
        (Transformation|SetRelativeRotation (Variables|Default|GetTree) (Variables|State|GetOriginalRotation) false false)
        (Timeline|VisibilityAnimation ReverseFromEnd)
        (else
          (CallFunction|SetActivated false))))))

(event EventInteractionRequested
  (params (InController :type Controller%20Object%20Reference))
  (|CallParentFunction InController)
  (Audio|PlaySoundatLocation "/Game/Sounds/Environment/TreeFall.TreeFall" "0, 0, 0" "0, 0, 0" 1.0 1.0 0.0 0 0 0)
  (bind _ratio (Timeline|TreeFallAnimation PlayFromStart)
    (:Update
      (Transformation|SetRelativeRotation (Variables|Default|GetTree) (Math|Rotator|CombineRotators (Variables|State|GetOriginalRotation) (Math|Rotator|MakeRotator 0.0 (* (- -9e+01 (.Pitch (Math|Rotator|BreakRotator (Variables|State|GetOriginalRotation)))) _ratio) 0.0)) false false))
    (:Finished
      (Utilities|Time|SetTimerbyEvent (EventDispatchers|CreateEvent :!event Custom|RespawnTrap) (Variables|Constant|GetRespawnTime)))))

(event EventBeginPlay
  (Utilities|FlowControl|Sequence
    (:then_0
      (if (Variables|Constant|GetApplyEffectByHit)
        (Collision|SetCollisionEnabled (Variables|Default|GetTree) "QueryAndPhysics")
        (Collision|SetCollisionEnabled (Variables|Default|GetBox) "NoCollision")
        (else
          (Collision|SetCollisionEnabled (Variables|Default|GetTree) "NoCollision")
          (Collision|SetCollisionEnabled (Variables|Default|GetBox) "QueryOnly"))))
    (:then_1
      (bind _returnvalue (Rendering|Material|CreateDynamicMaterialInstance "/Game/Procedural_Ecosystem/Materials/M_birch_bark1_Inst.M_birch_bark1_Inst" "None" :!class /Script/Engine.KismetMaterialLibrary))
      (Variables|State|SetMaterial _returnvalue)
      (for _index (range 0 2)
        (Rendering|Material|SetMaterial (Variables|Default|GetTree) _index (Variables|State|GetMaterial))))))

(fn ConstructionScript
  (Variables|State|SetOriginalRotation (Variables|/Script/Engine.SceneComponent|GetRelativeRotation (Variables|Default|GetTree))))