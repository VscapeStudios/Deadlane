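; An action volume that plays a configurable sound in the world when its FireAction event fires.
; FireAction composes the SoundTransform offset with the actor's transform, so the sound's location and rotation are relative to the volume.
; It plays the sound there with the configured attenuation and concurrency overrides.
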(event EventBeginPlay
  (|CallParentFunction) ; This node is disabled and will not be called.\nDrag off pins to build functionality.
)

(event Collision|EventActorBeginOverlap
  (params (OtherActor :type Actor%20Object%20Reference))
  (|CallParentFunction OtherActor) ; This node is disabled and will not be called.\nDrag off pins to build functionality.
)

(event EventTick
  (params (DeltaSeconds :type Float%20%28single-precision%29))
  (|CallParentFunction DeltaSeconds) ; This node is disabled and will not be called.\nDrag off pins to build functionality.
)

(event EventFireAction
  (params (InstigatorKart :type DE%20Ghost%20Kart%20Object%20Reference))
  (bind _returnvalue (Transformation|GetActorTransform))
  (bind _soundtransform (Variables|Default|GetSoundTransform))
  (bind _returnvalue_2 (Math|Transform|ComposeTransforms _soundtransform _returnvalue))
  (bind (_location _rotation) (Math|Transform|BreakTransform _returnvalue_2))
  (Audio|PlaySoundatLocation (Variables|Default|GetSound) _location _rotation 1.0 1.0 0.0 (Variables|Default|GetAttenuationOverride) (Variables|Default|GetConcurrencyOverride) 0))

(fn ConstructionScript
  (|CallParentFunction))