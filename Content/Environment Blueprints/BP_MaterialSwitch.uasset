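; BP_MaterialSwitch is an environment trigger that swaps the slot 0 material on a list of meshes while its Box is overlapped.
; The construction script caches each mesh's original material in DefaultMaterials, padding invalid entries to keep indices aligned.
; The first overlap applies the override Material, guarded by a Switched flag.
; When the last overlapping actor leaves, the flag clears and the cached materials are restored.
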(event OnComponentBeginOverlap(Box)
  (params (OverlappedComponent :type Primitive%20Component%20Object%20Reference) (OtherActor :type Actor%20Object%20Reference) (OtherComp :type Primitive%20Component%20Object%20Reference) (OtherBodyIndex :type Integer) (bFromSweep :type Boolean) (SweepResult :type Hit%20Result%20Structure%20%28by%20ref%29))
  (if (not (Variables|State|GetbSwitched))
    (Variables|State|SetbSwitched true)
    (for _array_element (Variables|Config|GetMeshes)
      (Utilities|IsValid _array_element
        (:Is%20Valid
          (Rendering|Material|SetMaterial (Variables|/Script/Engine.StaticMeshActor|GetStaticMeshComponent _array_element) 0 (Variables|Config|GetMaterial)))))))

(event OnComponentEndOverlap(Box)
  (params (OverlappedComponent :type Primitive%20Component%20Object%20Reference) (OtherActor :type Actor%20Object%20Reference) (OtherComp :type Primitive%20Component%20Object%20Reference) (OtherBodyIndex :type Integer))
  (if (== (Utilities|Array|Length (Collision|GetOverlappingActors (Variables|Default|GetBox) 0 :!class /Script/Engine.PrimitiveComponent)) 0)
    (Variables|State|SetbSwitched false)
    (for (_array_element _array_index) (Variables|Config|GetMeshes)
      (Utilities|IsValid _array_element
        (:Is%20Valid
          (Rendering|Material|SetMaterial (Variables|/Script/Engine.StaticMeshActor|GetStaticMeshComponent _array_element) 0 (Utilities|Array|Get(acopy) (Variables|State|GetDefaultMaterials) _array_index)))))))

(fn ConstructionScript
  (for _array_element (Variables|Config|GetMeshes)
    (Utilities|IsValid _array_element
      (:Is%20Valid
        (Utilities|Array|Add (Variables|State|GetDefaultMaterials) (Rendering|Material|GetMaterial (Variables|/Script/Engine.StaticMeshActor|GetStaticMeshComponent _array_element) 0)))
      (:Is%20Not%20Valid
        (Utilities|Array|Add (Variables|State|GetDefaultMaterials) 0)))))