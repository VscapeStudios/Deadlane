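; Demo triggerable actor for action volumes that plays scripted screen and glitch effects when a kart fires an action tag.
; Telly Go Crazy and Telly Go Sleep drive timelines that blend two post-process components.
; Glitch runs timelines animating Cham's pixel dissolve and glitch parameters.
; Camera cutscene, kart attach and detach, and sound logic remain disconnected, so Tick's look-at camera interpolation is never enabled here.
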(event EventBeginPlay
  (Variables|Default|SetRestTransform (Transformation|GetActorTransform)))

(event EventOnActionFired
  (params (ActionTag :type Name :default "None") (InstigatorKart :type DE%20Ghost%20Kart%20Object%20Reference))
  (bind _cham (Variables|Default|GetCham))
  (bind _output_get (Variables|Default|SetInstigatorKart InstigatorKart))
  (Utilities|IsValid _output_get
    (:Is%20Valid
      (Development|PrintString (Utilities|String|Append "New Action: " (Utilities|String|ToString(Name) ActionTag)) false)
      (switch name ActionTag
        (:TellyGoCrazy
          (bind _newtrack_0 (Timeline|Timeline_0 Play)
            (:Update
              (Variables|/Script/Engine.PostProcessComponent|SetBlendWeight (Variables|Default|GetPostProcess1) _newtrack_0))))
        (:TellyGoSleep
          (bind (_direction _newtrack_0_2 _newtrack_1) (Timeline|Timeline_1 Play)
            (:Update
              (Variables|/Script/Engine.PostProcessComponent|SetBlendWeight (Variables|Default|GetPostProcess2) _newtrack_0_2)
              (Variables|/Script/Engine.PostProcessComponent|SetBlendWeight (Variables|Default|GetPostProcess1) _newtrack_1))))
        (:Glitch
          (bind _newtrack_0_3 (Timeline|Timeline_2 Play)
            (:Update
              (Variables|/Game/Chameleon/Chameleon.Chameleon_C|SetPixel%20Dissolve%20Intensity (Variables|Default|GetCham) _newtrack_0_3)
              (bind (_direction_2 _glitch_speed _glitch_lines _glitch_blocking _glitch_grid_distortion_power _glitch_grid_distortion_size _glitch_grid_distortion_speed) (Timeline|Timeline_3 Play)
                (:Update
                  (Variables|/Game/Chameleon/Chameleon.Chameleon_C|SetGlitch%20Grid%20Distortion%20Speed _cham _glitch_grid_distortion_speed)
                  (Variables|/Game/Chameleon/Chameleon.Chameleon_C|SetGlitch%20Blocking _cham _glitch_blocking)
                  (Variables|/Game/Chameleon/Chameleon.Chameleon_C|SetGlitch%20Speed _cham _glitch_speed)
                  (Variables|/Game/Chameleon/Chameleon.Chameleon_C|SetGlitch%20Lines _cham _glitch_lines)
                  (Variables|/Game/Chameleon/Chameleon.Chameleon_C|SetGlitch%20Grid%20Distortion%20Power _cham _glitch_grid_distortion_power)
                  (Variables|/Game/Chameleon/Chameleon.Chameleon_C|SetGlitch%20Grid%20Distortion%20Size _cham _glitch_grid_distortion_size))))))))))

(event EventTick
  (params (DeltaSeconds :type Float%20%28single-precision%29))
  (if (Variables|Default|GetInterpCamera)
    (Transformation|SetWorldLocationAndRotation (Variables|Default|GetCamera) (Variables|Default|GetInterpLocation) (Math|Rotator|MakeRotfromX (- (Transformation|GetWorldLocation (Variables|Default|GetCameraTarget)) (Transformation|GetWorldLocation (Variables|Default|GetCamera)))) false false)))

(fn ConstructionScript)