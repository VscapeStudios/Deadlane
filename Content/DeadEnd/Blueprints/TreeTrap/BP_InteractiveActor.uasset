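; BP_InteractiveActor is an actor in the TreeTrap folder that player and AI controllers can activate by interacting within its KeyPressTrigger volume.
; Trigger overlaps bind or unbind the pawn controller's OnInteractionRequested event and notify it of availability with the InteractionTag.
; An interaction request sets Activated, which withdraws availability from all overlapping pawns and blocks new offers until cleared.
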(event OnComponentBeginOverlap(KeyPressTrigger)
  (params (OverlappedComponent :type Primitive%20Component%20Object%20Reference) (OtherActor :type Actor%20Object%20Reference) (OtherComp :type Primitive%20Component%20Object%20Reference) (OtherBodyIndex :type Integer) (bFromSweep :type Boolean) (SweepResult :type Hit%20Result%20Structure%20%28by%20ref%29))
  (if (not (Variables|State|GetbActivated))
    (bind _controller (Utilities|GetPawnContoller OtherActor)
      (:Valid
        (CallFunction|SetInteractionAllowedforController _controller true)))))

(event OnComponentEndOverlap(KeyPressTrigger)
  (params (OverlappedComponent :type Primitive%20Component%20Object%20Reference) (OtherActor :type Actor%20Object%20Reference) (OtherComp :type Primitive%20Component%20Object%20Reference) (OtherBodyIndex :type Integer))
  (bind _controller (Utilities|GetPawnContoller OtherActor)
    (:Valid
      (CallFunction|SetInteractionAllowedforController _controller false))))

(event Custom|InteractionRequested
  (params (InController :type Controller%20Object%20Reference))
  (CallFunction|SetActivated true))

(event EventBeginPlay)

(event Collision|EventActorBeginOverlap
  (params (OtherActor :type Actor%20Object%20Reference)))

(event EventTick
  (params (DeltaSeconds :type Float%20%28single-precision%29)))

(fn ConstructionScript)

(fn SetInteractionAllowedforController
  (params (InController :type Controller%20Object%20Reference) (bNewAvailable :type Boolean))
  (Utilities|FlowControl|Sequence
    (:then_0
      (bind _asdead_end_player_controller (Utilities|Casting|CastToDeadEnd_PlayerController InController))
      (LocalVariables|SetPlayerController _asdead_end_player_controller)
      (if bNewAvailable
        (EventDispatchers|BindEventtoOnInteractionRequested (LocalVariables|GetPlayerController) (EventDispatchers|CreateEvent :!event Custom|InteractionRequested))
        (else
          (EventDispatchers|UnbindEventfromOnInteractionRequested (LocalVariables|GetPlayerController) (EventDispatchers|CreateEvent :!event Custom|InteractionRequested))))
      (Default|NotifyInteractionAvailabilityChanged (LocalVariables|GetPlayerController) (Variables|Interaction|GetInteractionTag) bNewAvailable))
    (:then_1
      (bind _asdead_end_aicontoller (Utilities|Casting|CastToDeadEnd_AIContoller InController))
      (LocalVariables|SetAIController _asdead_end_aicontoller)
      (if bNewAvailable
        (EventDispatchers|BindEventtoOnInteractionRequested (LocalVariables|GetAIController) (EventDispatchers|CreateEvent :!event Custom|InteractionRequested))
        (else
          (EventDispatchers|UnbindEventfromOnInteractionRequested (LocalVariables|GetAIController) (EventDispatchers|CreateEvent :!event Custom|InteractionRequested))))
      (Default|NotifyInteractionAvailabilityChanged (LocalVariables|GetAIController) (Variables|Interaction|GetInteractionTag) bNewAvailable))))

(fn SetInteractionAllowedforOverlappers
  (params (bNewAllowed :type Boolean))
  (for _array_element (Collision|GetOverlappingActors (Variables|Default|GetKeyPressTrigger) "/Script/Engine.Pawn" :!class /Script/Engine.PrimitiveComponent)
    (bind _controller (Utilities|GetPawnContoller _array_element)
      (:Valid
        (CallFunction|SetInteractionAllowedforController _controller bNewAllowed)))))

(fn SetActivated
  (params (bNewActivated :type Boolean))
  (Variables|State|SetbActivated bNewActivated)
  (CallFunction|SetInteractionAllowedforOverlappers (not bNewActivated)))