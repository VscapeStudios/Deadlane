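; BP_TellyCue is a cue actor that blends the level's exponential height fog toward target settings alongside audio.
; On BeginPlay it caches the first fog component's density and height falloff, then starts audio and a timeline that drives both fog values and volume.
; BeginFadeOut waits a configurable delay, runs a second timeline over the same values, then destroys the actor.
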(event Custom|StartFadeIn
  (Utilities|IsValid (Variables|Default|GetFog)
    (:Is%20Valid
      (Audio|Components|Audio|Play (Variables|Default|GetAudio) 0.0)
      (bind _blendalpha (Timeline|FogAlphaTimeline PlayFromStart)
        (:Update
          (Class|ExponentialHeightFogComponent|SetFogDensity (Variables|Default|GetFog) (Math|Float|Lerp (Variables|Default|GetFogDencityCache) (Variables|Default|GetTargetFogDencity) _blendalpha))
          (Class|ExponentialHeightFogComponent|SetFogHeightFalloff (Variables|Default|GetFog) (Math|Float|Lerp (Variables|Default|GetFogHeightFalloffCache) (Variables|Default|GetTargetFogHeightFalloff) _blendalpha))
          (Audio|Components|Audio|SetVolumeMultiplier (Variables|Default|GetAudio) _blendalpha :!class /Script/Engine.AudioComponent))))))

(event Custom|BeginFadeOut
  (Utilities|FlowControl|Delay (Variables|Default|GetDelayBeforeFadeOut))
  (Utilities|IsValid (Variables|Default|GetFog)
    (:Is%20Valid
      (bind _blendalpha (Timeline|Timeline_0 PlayFromStart)
        (:Update
          (Class|ExponentialHeightFogComponent|SetFogDensity (Variables|Default|GetFog) (Math|Float|Lerp (Variables|Default|GetFogDencityCache) (Variables|Default|GetTargetFogDencity) _blendalpha))
          (Class|ExponentialHeightFogComponent|SetFogHeightFalloff (Variables|Default|GetFog) (Math|Float|Lerp (Variables|Default|GetFogHeightFalloffCache) (Variables|Default|GetTargetFogHeightFalloff) _blendalpha))
          (Audio|Components|Audio|SetVolumeMultiplier (Variables|Default|GetAudio) _blendalpha :!class /Script/Engine.AudioComponent))
        (:Finished
          (Actor|DestroyActor))))))

(event EventBeginPlay
  (Utilities|FlowControl|Sequence
    (:then_0
      (bind _outactors (Actor|GetAllActorsOfClass "/Script/Engine.ExponentialHeightFog"))
      (if (> (Utilities|Array|Length _outactors) 0)
        (bind _output_get (Variables|Default|SetFog (Variables|/Script/Engine.ExponentialHeightFog|GetComponent (Utilities|Array|Get(acopy) _outactors))))
        (Variables|Default|SetFogDencityCache (Variables|/Script/Engine.ExponentialHeightFogComponent|GetFogDensity _output_get))
        (Variables|Default|SetFogHeightFalloffCache (Variables|/Script/Engine.ExponentialHeightFogComponent|GetFogHeightFalloff _output_get))))
    (:then_1
      (CallFunction|StartFadein))))

(event Collision|EventActorBeginOverlap
  (params (OtherActor :type Actor%20Object%20Reference)))

(event EventTick
  (params (DeltaSeconds :type Float%20%28single-precision%29)))

(fn ConstructionScript)