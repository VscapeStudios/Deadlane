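; BP_Tellydonotuse is a player-controllable Telly character with basic movement and a look-up animation, named as not for use.
; Forward and Turn axis inputs add movement along the forward and right vectors of the actor's yaw, so Turn moves sideways without directly rotating.
; Pressing Handbrake plays the AM_LookUp montage on the mesh.
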(event Input|ActionEvents|InputActionHandbrake
  (params (Key :type Key%20Structure))
  (:Pressed
    (Animation|Montage|PlayMontage (Variables|Character|GetMesh) "/Game/Characters/Telly/AM_LookUp.AM_LookUp")))

(event Input|AxisEvents|InputAxisForward
  (params (AxisValue :type Float%20%28single-precision%29))
  (Pawn|Input|AddMovementInput (Math|Vector|GetForwardVector (Math|Rotator|MakeRotator 0.0 0.0 (.Yaw (Math|Rotator|BreakRotator (Transformation|GetActorRotation))))) AxisValue false))

(event Input|AxisEvents|InputAxisTurn
  (params (AxisValue :type Float%20%28single-precision%29))
  (Pawn|Input|AddMovementInput (Math|Vector|GetRightVector (Math|Rotator|MakeRotator 0.0 0.0 (.Yaw (Math|Rotator|BreakRotator (Transformation|GetActorRotation))))) AxisValue false))

(fn ConstructionScript)