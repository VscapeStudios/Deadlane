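; BP_ActionVolume_DemoActor is a demo actor that gives visual and audio feedback when its FireAction event is called, presumably by an action volume.
; FireAction turns both static meshes red, shows two point lights, plays an attenuated sound at the actor's location and attaches a flare particle effect to each light.
; It has no active tick, overlap or construction logic of its own, and nothing in it reverts the change.
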(event EventBeginPlay
  (|CallParentFunction) ; This node is disabled and will not be called.\nDrag off pins to build functionality.
)

(event Collision|EventActorBeginOverlap
  (params (OtherActor :type Actor%20Object%20Reference))
  (|CallParentFunction OtherActor) ; This node is disabled and will not be called.\nDrag off pins to build functionality.
)

(event EventTick
  (params (DeltaSeconds :type Float%20%28single-precision%29))
  (|CallParentFunction DeltaSeconds) ; This node is disabled and will not be called.\nDrag off pins to build functionality.
)

(event EventFireAction
  (params (InstigatorKart :type DE%20Ghost%20Kart%20Object%20Reference))
  (Utilities|FlowControl|Sequence
    (:then_0
      (Rendering|Material|SetMaterial (Variables|Default|GetStaticMesh) 0 "/Game/TestsAssets/MI_Red.MI_Red"))
    (:then_1
      (Rendering|SetVisibility (Variables|Default|GetPointLight2) true false))
    (:then_2
      (Audio|PlaySoundatLocation "/Engine/EditorSounds/GamePreview/StartPlayInEditor.StartPlayInEditor" (Transformation|GetActorLocation) "0,0.000000, 0" 1.0 1.0 0.0 "/Game/Sounds/Kart_Sounds/SA_Otherkarts.SA_OtherKarts" 0 0))
    (:then_3
      (Effects|SpawnEmitterAttached "/Game/Flare_FX/P_Flare_Fast_LargeSpawn.P_Flare_Fast_LargeSpawn" (Variables|Default|GetPointLight2) "None" "0, 0,0.000000")
      (Effects|SpawnEmitterAttached "/Game/Flare_FX/P_Flare_Fast_LargeSpawn.P_Flare_Fast_LargeSpawn" (Variables|Default|GetPointLight1) "None"))))

(fn ConstructionScript
  (|CallParentFunction))