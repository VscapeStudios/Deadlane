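; BP_PlayerTV is a TV prop that plays media on its screen and switches back to blank footage.
; BeginPlay and five identical EventBeginPlay variants bind a media texture to a dynamic screen material and open the blank source.
; Numbered TurnOn events open separate image sources on their own media players, while every TurnOff blanks the main player.
; All these switch events toggle the point light; plain TurnOn only opens the main source.
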(event Custom|TurnOn1
  (Media|MediaPlayer|OpenSource (Variables|Default|GetMediaPlayer_0) "/Game/Movies/NewImgMediaSource1.NewImgMediaSource1")
  (Rendering|ToggleVisibility (Variables|Default|GetPointLight) false))

(event Custom|TurnOff5
  (Media|MediaPlayer|OpenSource (Variables|Default|GetMediaPlayer) "/Game/Movies/BlankFootage.BlankFootage")
  (Rendering|ToggleVisibility (Variables|Default|GetPointLight) false))

(event Custom|TurnOff2
  (Media|MediaPlayer|OpenSource (Variables|Default|GetMediaPlayer) "/Game/Movies/BlankFootage.BlankFootage")
  (Rendering|ToggleVisibility (Variables|Default|GetPointLight) false))

(event Custom|EventBeginPlay2
  (bind _staticmesh (Variables|Default|GetStaticMesh))
  (bind _returnvalue (Rendering|Material|CreateDynamicMaterialInstance _staticmesh 1 (Rendering|Material|GetMaterial _staticmesh 1) "None" :!class /Script/Engine.PrimitiveComponent))
  (bind _output_get (Variables|Default|SetDMI_Screen _returnvalue))
  (Rendering|Material|SetTextureParameterValue _output_get "MediaTexture" (Variables|Default|GetTexture))
  (Media|MediaPlayer|OpenSource (Variables|Default|GetMediaPlayer) "/Game/Movies/BlankFootage.BlankFootage"))

(event Custom|TurnOn4
  (Media|MediaPlayer|OpenSource (Variables|Default|GetMediaPlayer_3) "/Game/Movies/NewImgMediaSource4.NewImgMediaSource4")
  (Rendering|ToggleVisibility (Variables|Default|GetPointLight) false))

(event Custom|TurnOff3
  (Media|MediaPlayer|OpenSource (Variables|Default|GetMediaPlayer) "/Game/Movies/BlankFootage.BlankFootage")
  (Rendering|ToggleVisibility (Variables|Default|GetPointLight) false))

(event Custom|EventBeginPlay5
  (bind _staticmesh (Variables|Default|GetStaticMesh))
  (bind _returnvalue (Rendering|Material|CreateDynamicMaterialInstance _staticmesh 1 (Rendering|Material|GetMaterial _staticmesh 1) "None" :!class /Script/Engine.PrimitiveComponent))
  (bind _output_get (Variables|Default|SetDMI_Screen _returnvalue))
  (Rendering|Material|SetTextureParameterValue _output_get "MediaTexture" (Variables|Default|GetTexture))
  (Media|MediaPlayer|OpenSource (Variables|Default|GetMediaPlayer) "/Game/Movies/BlankFootage.BlankFootage"))

(event Custom|TurnOn5
  (Media|MediaPlayer|OpenSource (Variables|Default|GetMediaPlayer_4) "/Game/Movies/NewImgMediaSource5.NewImgMediaSource5")
  (Rendering|ToggleVisibility (Variables|Default|GetPointLight) false))

(event Custom|TurnOn
  (Media|MediaPlayer|OpenSource (Variables|Default|GetMediaPlayer) (Variables|Default|GetMediaSource)))

(event Custom|TurnOff4
  (Media|MediaPlayer|OpenSource (Variables|Default|GetMediaPlayer) "/Game/Movies/BlankFootage.BlankFootage")
  (Rendering|ToggleVisibility (Variables|Default|GetPointLight) false))

(event Custom|EventBeginPlay3
  (bind _staticmesh (Variables|Default|GetStaticMesh))
  (bind _returnvalue (Rendering|Material|CreateDynamicMaterialInstance _staticmesh 1 (Rendering|Material|GetMaterial _staticmesh 1) "None" :!class /Script/Engine.PrimitiveComponent))
  (bind _output_get (Variables|Default|SetDMI_Screen _returnvalue))
  (Rendering|Material|SetTextureParameterValue _output_get "MediaTexture" (Variables|Default|GetTexture))
  (Media|MediaPlayer|OpenSource (Variables|Default|GetMediaPlayer) "/Game/Movies/BlankFootage.BlankFootage"))

(event Custom|TurnOn2
  (Media|MediaPlayer|OpenSource (Variables|Default|GetMediaPlayer_1) "/Game/Movies/NewImgMediaSource2.NewImgMediaSource2")
  (Rendering|ToggleVisibility (Variables|Default|GetPointLight) false))

(event Custom|TurnOff
  (Media|MediaPlayer|OpenSource (Variables|Default|GetMediaPlayer) "/Game/Movies/BlankFootage.BlankFootage")
  (Rendering|ToggleVisibility (Variables|Default|GetPointLight) false))

(event Custom|TurnOff1
  (Media|MediaPlayer|OpenSource (Variables|Default|GetMediaPlayer) "/Game/Movies/BlankFootage.BlankFootage")
  (Rendering|ToggleVisibility (Variables|Default|GetPointLight) false))

(event Custom|EventBeginPlay1
  (bind _staticmesh (Variables|Default|GetStaticMesh))
  (bind _returnvalue (Rendering|Material|CreateDynamicMaterialInstance _staticmesh 1 (Rendering|Material|GetMaterial _staticmesh 1) "None" :!class /Script/Engine.PrimitiveComponent))
  (bind _output_get (Variables|Default|SetDMI_Screen _returnvalue))
  (Rendering|Material|SetTextureParameterValue _output_get "MediaTexture" (Variables|Default|GetTexture))
  (Media|MediaPlayer|OpenSource (Variables|Default|GetMediaPlayer) "/Game/Movies/BlankFootage.BlankFootage"))

(event Custom|TurnOn3
  (Media|MediaPlayer|OpenSource (Variables|Default|GetMediaPlayer_2) "/Game/Movies/NewImgMediaSource3.NewImgMediaSource3")
  (Rendering|ToggleVisibility (Variables|Default|GetPointLight) false))

(event Custom|EventBeginPlay4
  (bind _staticmesh (Variables|Default|GetStaticMesh))
  (bind _returnvalue (Rendering|Material|CreateDynamicMaterialInstance _staticmesh 1 (Rendering|Material|GetMaterial _staticmesh 1) "None" :!class /Script/Engine.PrimitiveComponent))
  (bind _output_get (Variables|Default|SetDMI_Screen _returnvalue))
  (Rendering|Material|SetTextureParameterValue _output_get "MediaTexture" (Variables|Default|GetTexture))
  (Media|MediaPlayer|OpenSource (Variables|Default|GetMediaPlayer) "/Game/Movies/BlankFootage.BlankFootage"))

(event EventBeginPlay
  (bind _staticmesh (Variables|Default|GetStaticMesh))
  (bind _returnvalue (Rendering|Material|CreateDynamicMaterialInstance _staticmesh 1 (Rendering|Material|GetMaterial _staticmesh 1) "None" :!class /Script/Engine.PrimitiveComponent))
  (bind _output_get (Variables|Default|SetDMI_Screen _returnvalue))
  (Rendering|Material|SetTextureParameterValue _output_get "MediaTexture" (Variables|Default|GetTexture))
  (Media|MediaPlayer|OpenSource (Variables|Default|GetMediaPlayer) "/Game/Movies/BlankFootage.BlankFootage"))

(fn ConstructionScript)