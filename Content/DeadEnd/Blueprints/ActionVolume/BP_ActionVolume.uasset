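; Base trigger volume that runs an action when a qualifying DEGhostKart overlaps its box, with FireAction left empty.
; CanFire gates firing by remaining uses, cooldown timer, prerequisite actions completed in DeadEnd_GameState, and a first-player, any-player or any-kart filter.
; CompleteAction decrements uses, starts the cooldown, records completion in the game state, and can destroy the volume once exhausted.
; The construction script sizes the box and optionally adds a tinted debug mesh.
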(event OnComponentBeginOverlap(Box)
  (params (OverlappedComponent :type Primitive%20Component%20Object%20Reference) (OtherActor :type Actor%20Object%20Reference) (OtherComp :type Primitive%20Component%20Object%20Reference) (OtherBodyIndex :type Integer) (bFromSweep :type Boolean) (SweepResult :type Hit%20Result%20Structure%20%28by%20ref%29))
  (bind _asdeghost_kart (Utilities|Casting|CastToDEGhostKart OtherActor))
  (if (CallFunction|CanFire _asdeghost_kart)
    (CallFunction|FireAction _asdeghost_kart)
    (CallFunction|CompleteAction)))

(event Custom|FireAction
  (params (InstigatorKart :type DE%20Ghost%20Kart%20Object%20Reference)))

(event EventBeginPlay)

(event Collision|EventActorBeginOverlap
  (params (OtherActor :type Actor%20Object%20Reference)))

(event EventTick
  (params (DeltaSeconds :type Float%20%28single-precision%29)))

(fn ConstructionScript
  (Components|Box|SetBoxExtent (Variables|Default|GetBox) (Variables|Config|GetBoxExtent) true)
  (if (or (Variables|Config|GetbDrawDebugInGame) (Variables|Config|GetbDrawDebug))
    (bind _returnvalue (AddComponent|AddStaticMeshComponent false))
    (Utilities|IsValid _returnvalue
      (:Is%20Valid
        (Transformation|SetRelativeScale3D _returnvalue (/ (Variables|Config|GetBoxExtent) 5e+01))
        (Development|SetHiddeninGame _returnvalue (not (Variables|Config|GetbDrawDebugInGame)) false)
        (bind _returnvalue_2 (Rendering|Material|CreateDynamicMaterialInstance "/Game/TestsAssets/MI_Translucent.MI_Translucent" "None" :!class /Script/Engine.KismetMaterialLibrary))
        (Rendering|Material|SetVectorParameterValue _returnvalue_2 "Color" (Variables|Config|GetDebugMeshColor) :!class /Script/Engine.MaterialInstanceDynamic)
        (Rendering|Material|SetMaterial _returnvalue 0 _returnvalue_2)))))

(fn CanFire
  (params (OverlappingKart :type DE%20Ghost%20Kart%20Object%20Reference))
  (if (Math|Boolean|ANDBoolean (Utilities|IsValid OverlappingKart) (!= (Variables|Config|GetActionsNum) 0) (not (CallFunction|IsinCooldown)))
    (if (> (Utilities|Array|Length (Variables|Config|GetDependOnActions)) 0)
      (bind _asdead_end_game_state (Utilities|Casting|CastToDeadEnd_GameState (Game|GetGameState))
        (:then
          (LocalVariables|SetGS _asdead_end_game_state)
          (LocalVariables|SetbAllDepenOnCompleted true)
          (bind _array_element (Utilities|Array|ForEachLoopwithBreak (Variables|Config|GetDependOnActions) :!label _label)
            (:LoopBody
              (if (not (Default|IsActionCompleted (LocalVariables|GetGS) _array_element))
                (LocalVariables|SetbAllDepenOnCompleted false)
                (goto _label Break)))
            (:Completed
              (if (LocalVariables|GetbAllDepenOnCompleted)
                (switch Utilities|FlowControl|Switch|SwitchonActionVolumeTriggerType (Variables|Config|GetFireFrom) :!label _label_2
                  (:NewEnumerator0
                    (return (== (Pawn|GetController OverlappingKart) (Game|GetPlayerController 0))))
                  (:NewEnumerator1
                    (return (not (Pawn|IsBotControlled OverlappingKart))))
                  (:NewEnumerator2
                    (return true)))
                (else
                  (return false))))))
        (:CastFailed
          (return false)))
      (else
        (goto _label_2)))
    (else
      (return false))))

(fn CompleteAction
  (Utilities|FlowControl|Sequence
    (:then_0
      (if (> (Variables|Config|GetActionsNum) 0)
        (Math|Integer|DecrementInt (Variables|Config|GetActionsNum))))
    (:then_1
      (if (and (!= (Variables|Config|GetActionsNum) 0) (> (Variables|Config|GetCooldown) 0.0))
        (bind _returnvalue (Utilities|Time|SetTimerbyFunctionName 0 "OnCooldownFinished" (Variables|Config|GetCooldown)))
        (Variables|Vars|SetCooldownTimer _returnvalue)))
    (:then_2
      (bind _asdead_end_game_state (Utilities|Casting|CastToDeadEnd_GameState (Game|GetGameState)))
      (Default|SetActionCompleted _asdead_end_game_state (Utilities|ResolveSoftReference self) true))
    (:then_3
      (if (== (Variables|Config|GetActionsNum) 0)
        (if (> (Variables|Config|GetLifeSpanAfterExhausted) 0.0)
          (Actor|SetLifeSpan (Variables|Config|GetLifeSpanAfterExhausted))
          (elif (== (Variables|Config|GetLifeSpanAfterExhausted) 0.0)
            (Actor|DestroyActor)))))))

(fn OnCooldownFinished
  (Utilities|Time|ClearandInvalidateTimerbyHandle (Variables|Vars|GetCooldownTimer)))

(fn IsinCooldown
  (return (Utilities|Time|IsTimerActivebyHandle (Variables|Vars|GetCooldownTimer))))